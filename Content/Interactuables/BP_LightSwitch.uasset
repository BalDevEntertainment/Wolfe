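; Interactable light switch that toggles a spot light and its indirect lighting contribution off and on.
; The construction script caches the referenced SpotLight's starting intensity.
; Each Interact fires two FlipFlops: one rewrites LightIntensity's post-process settings for indirect light, the other sets the spot light to zero or its cached intensity.
; The first interaction switches both off, so the light is assumed to start on.
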(event EventBeginPlay)

(event Collision|EventActorBeginOverlap
  (params (OtherActor :type Actor%20Object%20Reference)))

(event EventTick
  (params (DeltaSeconds :type Float%20%28single-precision%29)))

(event EventInteract
  (Utilities|FlowControl|Sequence
    (:then_0
      ;[1 1 1] Change Indirectional Light
      (bind _isa (Utilities|FlowControl|FlipFlop)
        (:A
          _)
        (:B
          _))
      (Variables|/Script/Engine.PostProcessVolume|SetSettings (Variables|Default|GetLightIntensity) (Utilities|Struct|MakePostProcessSettings (Math|Float|SelectFloat 0.0 1.0 _isa))))
    (:then_1
      ;[1 1 1] Change Direct Lightning
      (bind _isa_2 (Utilities|FlowControl|FlipFlop)
        (:A
          _)
        (:B
          _))
      (Rendering|Components|Light|SetIntensity (Variables|/Script/Engine.SpotLight|GetSpotLightComponent (Variables|Default|GetSpotLight)) (Math|Float|SelectFloat 0.0 (Variables|Default|GetStartingIntensity) _isa_2)))))

(fn ConstructionScript
  (Variables|Default|SetStartingIntensity (Variables|/Script/Engine.LightComponentBase|GetIntensity (Variables|/Script/Engine.Light|GetLightComponent (Variables|Default|GetSpotLight)))))